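; GM_Main is a game mode Blueprint that spawns the asteroids when play begins.
; It waits tick by tick until the viewport reports a non-zero size, then deprojects screen points from the first player controller to build a world-space box.
; It spawns BP_Asteroid actors at random points in that box at a fixed height, stores them in the Asteroids array and prints a completion message.
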(event Custom|SpawnAsteroids
  (bind _returnvalue (Viewport|GetViewportSize))
  (bind _returnvalue_2 (Game|GetPlayerController 0))
  (bind _divideamount (Variables|Default|GetdivideAmount))
  (bind _returnvalue_3 (/ _returnvalue _divideamount))
  (bind (_x _y) (Math|Vector2D|BreakVector2D _returnvalue_3))
  (bind _worldlocation (Class|PlayerController|DeprojectScreenPositiontoWorld _returnvalue_2 _x _y))
  (if (Utilities|Operators|NotEqual(!=) :A _returnvalue) :!label _label
    (for _index (range 0 (- (Variables|Default|GetMaxAsteroidsCount) 1))
      (Variables|Default|SetRandPoint (Math|Random|RandomPointinBoundingBox _worldlocation (- _worldlocation (.WorldLocation (Class|PlayerController|DeprojectScreenPositiontoWorld _returnvalue_2 0.0 0.0)))))
      (bind _returnvalue_4 (Game|SpawnActorfromClass "/Game/BP_Asteroid.BP_Asteroid_C" (Math|Transform|MakeTransform (Math|Vector|MakeVector (.X (Math|Vector|BreakVector (Variables|Default|GetRandPoint))) (.Y (Math|Vector|BreakVector (Variables|Default|GetRandPoint))) 92.0)) "Undefined" "MultiplyWithRoot" 0 0))
      (Utilities|Array|Add (Variables|Default|GetAsteroids) _returnvalue_4))
    (Development|PrintString "Asteroids finished spawning" true true "(R=0.099559,G=1.000000,B=0.000000,A=1.000000)" 1e+01)
    (else
      (Utilities|FlowControl|DelayUntilNextTick)
      (goto _label))))

(event EventBeginPlay
  (|CallParentFunction)
  (CallFunction|SpawnAsteroids))

(fn ConstructionScript)