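; BP_Ship is a ship steered by physics forces applied to its static mesh.
; Rotate applies yaw torque scaled by an input value and RotationForce, and Thrust applies an impulse along the actor's forward vector scaled by ThrustForce.
; Tick only calls the parent, and leftover debug nodes, including a sphere at the Muzzle component, are disconnected.
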(event Collision|EventActorBeginOverlap
  (params (OtherActor :type Actor%20Object%20Reference)))

(event EventThrust
  (Physics|AddImpulse (Variables|Default|GetStaticMesh) (* (Transformation|GetActorForwardVector) (Variables|Default|GetThrustForce)) "None" false))

(event EventRotate
  (params (Value :type Float%20%28single-precision%29))
  (Class|PrimitiveComponent|AddTorqueinRadians (Variables|Default|GetStaticMesh) (Math|Vector|MakeVector 0.0 0.0 (* (Variables|Default|GetRotationForce) Value)) "None" false))

(event EventTick
  (params (DeltaSeconds :type Float%20%28single-precision%29))
  (|CallParentFunction DeltaSeconds))

(fn ConstructionScript)