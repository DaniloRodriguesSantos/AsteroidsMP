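; Actor component that keeps its owner inside the arena by wrapping it to the opposite edge when it leaves on X or Y.
; Each Tick compares the owner's location to the Origin and Extents from GetArenaBoundaries, both passed through KillZ and treated as opposite corners.
; Chained branches move the owner with SetActorLocation without sweep, correcting at most one axis per frame and keeping Z unchanged.
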(event EventBeginPlay)

(event EventTick
  (params (DeltaSeconds :type Float%20%28single-precision%29))
  (bind (_origin _extents) (CallFunction|GetArenaBoundaries))
  (bind _returnvalue (Components|GetOwner))
  (bind _returnvalue_2 (Components|GetOwner))
  (bind _returnvalue_3 (Components|GetOwner))
  (bind _returnvalue_4 (Components|GetOwner))
  (bind _returnvalue_5 (Components|GetOwner))
  (bind _returnvalue_6 (CallFunction|KillZ _origin))
  (bind _returnvalue_7 (Transformation|GetActorLocation _returnvalue_5))
  (bind _returnvalue_8 (Transformation|GetActorLocation _returnvalue))
  (bind _returnvalue_9 (Transformation|GetActorLocation _returnvalue_2))
  (bind _returnvalue_10 (Transformation|GetActorLocation _returnvalue_4))
  (bind _returnvalue_11 (Transformation|GetActorLocation _returnvalue_3))
  (bind _returnvalue_12 (CallFunction|KillZ _extents))
  (bind (_x _y _z) (Math|Vector|BreakVector _returnvalue_7))
  (bind (_x_2 _y_2) (Math|Vector|BreakVector _returnvalue_12))
  (bind (_x_3 _y_3 _z_2) (Math|Vector|BreakVector _returnvalue_8))
  (bind (_x_4 _y_4 _z_3) (Math|Vector|BreakVector _returnvalue_9))
  (bind (_x_5 _y_5 _z_4) (Math|Vector|BreakVector _returnvalue_10))
  (bind _returnvalue_13 (CallFunction|KillZ _returnvalue_11))
  (bind (_x_6 _y_6) (Math|Vector|BreakVector _returnvalue_6))
  (bind (_x_7 _y_7) (Math|Vector|BreakVector _returnvalue_13))
  (if (> _x_7 _x_6)
    (Transformation|SetActorLocation _returnvalue (Math|Vector|MakeVector _x_2 _y_3 _z_2) false false)
    (elif (< _x_7 _x_2)
      (Transformation|SetActorLocation _returnvalue_2 (Math|Vector|MakeVector _x_6 _y_4 _z_3) false false)
      (elif (< _y_7 _y_6)
        (Transformation|SetActorLocation _returnvalue_4 (Math|Vector|MakeVector _x_5 _y_2 _z_4) false false)
        (elif (> _y_7 _y_2)
          (Transformation|SetActorLocation _returnvalue_5 (Math|Vector|MakeVector _x _y_6 _z) false false))))))